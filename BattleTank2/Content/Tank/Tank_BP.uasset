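; Tank Blueprint that sets up the tank's barrel reference and player camera aiming.
; On BeginPlay it passes the TankBarrel component to SetBarrelReference.
; Aim axis inputs orbit the camera through a two-part rig, yawing AzimuthGimbal and pitching SpringArm separately in local space.
; Both rotations scale by world delta time and a fixed speed, with no pitch clamping.
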(event EventBeginPlay
  (Class|Tank|SetBarrelReference (Variables|Default|GetTankBarrel)))

(event Input|AxisEvents|InputAxisAimAzimuth
  (params (AxisValue :type Float%20%28single-precision%29))
  ;[1 1 1] Camera Input Binding
  (Transformation|AddLocalRotation (Variables|Default|GetAzimuth%20Gimbal) (Math|Rotator|MakeRotator 0.0 0.0 (* AxisValue (Utilities|Time|GetWorldDeltaSeconds) 5e+01)) false false))

(event Input|AxisEvents|InputAxisAimElevation
  (params (AxisValue :type Float%20%28single-precision%29))
  ;[1 1 1] Camera Input Binding
  (Transformation|AddLocalRotation (Variables|Default|GetSpringArm) (Math|Rotator|MakeRotator 0.0 (* AxisValue (Utilities|Time|GetWorldDeltaSeconds) 5e+01) 0.0) false false))

(fn ConstructionScript)